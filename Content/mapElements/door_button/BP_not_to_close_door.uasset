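; Door actor that opens when a player or box overlaps it and has no logic to close again.
; BeginPlay caches the closed and target world locations and sets the timeline's play rate from a variable.
; Overlap by BP_Box or BP_Player plays the DoorMove timeline, which lerps the door toward the DoorMoveTo location without sweeping.
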(event `self.ReceiveBeginPlay`
  (set `self.backDoorLocation` (`SceneComponent.K2_GetComponentLocation` (`self.door`)))
  (set `self.moveDoorLocation` (`SceneComponent.K2_GetComponentLocation` (`self.doorMoveTo`)))
  (`TimelineComponent.SetPlayRate` (`self.doorMove`) (`self.NewVar`)))

(event `self.ReceiveActorBeginOverlap`
  (params (OtherActor :type "Actor Object Reference"))
  (`|ExecutionSequence`
    (:`then_0`
      (cast `/Game/mapElements/BP_Box` OtherActor)
      (bind (_direction _newtrack_0) (`Timeline|doorMove` :!label _label)
        (:`Update`
          (`SceneComponent.K2_SetWorldLocation` (`self.door`) (`KismetMathLibrary.VLerp` (`self.backDoorLocation`) (`self.moveDoorLocation`) _newtrack_0) false false))))
    (:`then_1`
      (cast `/Game/player/BP_Player` OtherActor)
      (goto _label))))

(fn `UserConstructionScript`)