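; BP_teleport_to_next_lvl is a map trigger that moves the player to the next level's location once they have enough points.
; On overlap it compares the player's Point with PointToTp, teleports player pawn 0 to TpLocation, then resets Point and increments OnLVL on the overlapping BP_Player.
; The player reference and TpLocation (from the TeleportLocation component) are cached after that check, so the check uses values from an earlier overlap.
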(event `self.ReceiveActorBeginOverlap`
  (params (OtherActor :type "Actor Object Reference"))
  (`|ExecutionSequence`
    (:`then_0`
      (if (>= (`/Game/player/BP_Player.point` (stale _asbp_player_2)) (`self.point to tp`))
        (`self.K2_TeleportTo` :`self` (`GameplayStatics.GetPlayerPawn` 0) :`DestLocation` (stale _output_get))
        (bind _asbp_player (cast `/Game/player/BP_Player` OtherActor))
        (`|ExecutionSequence`
          (:`then_0`
            (set `/Game/player/BP_Player.point` 0 _asbp_player))
          (:`then_1`
            (`/Engine/EditorBlueprintResources/StandardMacros.IncrementInt` (`/Game/player/BP_Player.onLVL` _asbp_player))))))
    (:`then_1`
      (bind _output_get (set `self.tp_location` (`SceneComponent.K2_GetComponentLocation` (`self.teleportLocation`)))))
    (:`then_2`
      (bind _asbp_player_2 (cast `/Game/player/BP_Player` OtherActor)))))

(fn `UserConstructionScript`)