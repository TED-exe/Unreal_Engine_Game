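; Automatic moving platform actor that slides its Plane component toward an EndPoint component once play begins.
; On BeginPlay it sets the PaltformMove timeline's play rate from Speed, caches both components' world locations as start and end, then plays the timeline.
; Each timeline update lerps the Plane's world location between those points using the track value, without sweep.
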(event `self.ReceiveBeginPlay`
  (`|ExecutionSequence`
    (:`then_0`
      (`TimelineComponent.SetPlayRate` (`self.paltformMove`) (`self.speed`)))
    (:`then_1`
      (set `self.startLocation` (`SceneComponent.K2_GetComponentLocation` (`self.Plane`)))
      (set `self.endLocation` (`SceneComponent.K2_GetComponentLocation` (`self.endPoint`)))
      (bind (_direction _newtrack_0) (`Timeline|paltformMove`)
        (:`Update`
          (`SceneComponent.K2_SetWorldLocation` (`self.Plane`) (`KismetMathLibrary.VLerp` (`self.startLocation`) (`self.endLocation`) _newtrack_0) false false))))))

(fn `UserConstructionScript`)