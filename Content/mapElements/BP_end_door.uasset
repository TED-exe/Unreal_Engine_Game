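; BP_end_door is a level exit door actor that removes itself once the player has enough points on the matching level.
; Each tick it compares the player's Point against its IsPoint threshold and the player's OnLVL against its IsLVL, destroying itself when both pass.
; The BP_Player reference is refreshed by a cast on every tick, after the check runs, so the first check precedes any assignment.
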(event `self.ReceiveTick`
  (params (DeltaSeconds :type "Float (single-precision)"))
  (`|ExecutionSequence`
    (:`then_0`
      (if (>= (`/Game/player/BP_Player.point` (stale _asbp_player)) (`self.isPoint`))
        (if (== (`self.isLVL`) (`/Game/player/BP_Player.onLVL` (stale _asbp_player)))
          (`self.K2_DestroyActor`))))
    (:`then_1`
      (bind _asbp_player (cast `/Game/player/BP_Player` (`GameplayStatics.GetPlayerPawn` 0))))))

(fn `UserConstructionScript`)