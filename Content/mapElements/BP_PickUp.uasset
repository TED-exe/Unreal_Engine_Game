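; BP_PickUp is a collectible map element that the player picks up by touching it.
; It rotates in local space each tick using roll, pitch and yaw speeds scaled by delta time.
; On overlap with a BP_Player, it destroys itself and increments that player's Point count.
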(event `self.ReceiveTick`
  (params (DeltaSeconds :type "Float (single-precision)"))
  (`self.K2_AddActorLocalRotation` (* (`KismetMathLibrary.MakeRotator` (`self.rollSpeed`) (`self.pitchSpeed`) (`self.yawSpeed`)) DeltaSeconds)))

(event `self.ReceiveActorBeginOverlap`
  (params (OtherActor :type "Actor Object Reference"))
  (bind _asbp_player (cast `/Game/player/BP_Player` OtherActor))
  (`self.K2_DestroyActor`)
  (`/Engine/EditorBlueprintResources/StandardMacros.IncrementInt` (`/Game/player/BP_Player.point` _asbp_player)))

(fn `UserConstructionScript`)