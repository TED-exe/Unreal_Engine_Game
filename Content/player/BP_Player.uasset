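; BP_Player is the player Blueprint, providing mouse-wheel camera zoom and a jump-readiness flag.
; The wheel steps an integer CameraPosition, clamped symmetrically to MaxCameraPosition, and Tick eases the spring arm length toward a default plus that step times a zoom increment.
; Any Hit event sets CanJump to true, while debug prints for level and point values are left unconnected.
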(event `InputAxisKey|MouseWheelAxis`
  (params (AxisValue :type "Float (single-precision)"))
  (bind _maxcameraposition (`self.maxCameraPosition`))
  (bind _maxcameraposition_2 (`self.maxCameraPosition`))
  ;[1 1 1] whhile scrolling
  (if (< AxisValue 0.0)
    (bind _result (`/Engine/EditorBlueprintResources/StandardMacros.IncrementInt` (`self.cameraPosition`))
      (:`  `
        (set `self.cameraPosition` (`KismetMathLibrary.Clamp` _result (* _maxcameraposition_2 -1) _maxcameraposition_2))))
    (elif (> AxisValue 0.0)
      (bind _result_2 (`/Engine/EditorBlueprintResources/StandardMacros.DecrementInt` (`self.cameraPosition`))
        (:`  `
          (set `self.cameraPosition` (`KismetMathLibrary.Clamp` _result_2 (* _maxcameraposition -1) _maxcameraposition)))))))

(event `self.ReceiveTick`
  (params (DeltaSeconds :type "Float (single-precision)"))
  ;[1 1 1] change arm leanght
  (`|ExecutionSequence`
    (:`then_0`
      (set `SpringArmComponent.TargetArmLength` (`KismetMathLibrary.FInterpTo` (`SpringArmComponent.TargetArmLength` (`self.SpringArm`)) (+ (`self.defaultSpiringArmLeangth`) (* (`self.cameraZoomDifference`) (`self.cameraPosition`))) DeltaSeconds 2.0) (`self.SpringArm`)))))

(event `self.ReceiveHit`
  (params (MyComp :type "PrimitiveComponent Object Reference") (Other :type "Actor Object Reference") (OtherComp :type "PrimitiveComponent Object Reference") (bSelfMoved :type Boolean) (HitLocation :type "Vector Structure") (HitNormal :type "Vector Structure") (NormalImpulse :type "Vector Structure") (Hit :type "HitResult Structure (by ref)"))
  (set `self.canJump` true))

(fn `UserConstructionScript`)