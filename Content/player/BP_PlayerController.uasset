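; Player controller for BP_Player, driving its sphere's movement and jump and its spring-arm camera.
; While right mouse is held, two Tick gates run RotateCamera, with clamped pitch, and RotatePlayer, which yaws the sphere.
; Vertical and Horizontal axes share one speed-scaled impulse, feeding one value into both world X and Y.
; Jump applies a velocity-change impulse and clears CanJump; the ground-check function is an empty stub.
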(event `self.ReceiveTick`
  (params (DeltaSeconds :type "Float (single-precision)"))
  ;[1 1 1] Comment
  (`|ExecutionSequence`
    (:`then_0`
      (`/Engine/EditorBlueprintResources/StandardMacros.Gate` true :!label _label
        (:`Exit`
          (`self.rotateCamera`))))
    (:`then_1`
      (`/Engine/EditorBlueprintResources/StandardMacros.Gate` true :!label _label_2
        (:`Exit`
          (`self.rotatePlayer`))))))

(event `Key|RightMouseButton`
  (params (Key :type "Key Structure"))
  ;[1 1 1] Comment
  (:`Pressed`
    (goto _label :!via `Open`))
  (:`Released`
    (goto _label :!via `Close`)))

(event `Key|RightMouseButton`
  (params (Key :type "Key Structure"))
  ;[1 1 1] Comment
  (:`Pressed`
    (goto _label_2 :!via `Open`))
  (:`Released`
    (goto _label_2 :!via `Close`)))

(event `InputAxis|Vertical`
  (params (AxisValue :type "Float (single-precision)"))
  ;[1 1 1] movemnt
  (bind _asbp_player (cast `/Game/player/BP_Player` (`GameplayStatics.GetPlayerPawn` 0) :!label _label_3))
  (`PrimitiveComponent.AddImpulse` (`/Game/player/BP_Player.Sphere` _asbp_player) (* (`KismetMathLibrary.MakeVector` AxisValue (stale `InputAxis|Horizontal` AxisValue)) (`self.Speed`)) "None" false))

(event `InputAxis|Horizontal`
  (params (AxisValue :type "Float (single-precision)"))
  ;[1 1 1] movemnt
  (goto _label_3))

(event `InputAction|Jump`
  (params (Key :type "Key Structure"))
  ;[1 1 1] Comment
  (:`Pressed`
    (bind _asbp_player (cast `/Game/player/BP_Player` (`GameplayStatics.GetPlayerPawn` 0)))
    (if (`/Game/player/BP_Player.canJump` _asbp_player)
      (`PrimitiveComponent.AddImpulse` (`/Game/player/BP_Player.Sphere` _asbp_player) (`KismetMathLibrary.MakeVector` 0.0 0.0 (`self.Jump Force`)) "None" true)
      (set `/Game/player/BP_Player.canJump` false _asbp_player))))

(fn `isGroundedChech`)

(fn `rotateCamera`
  (bind _asbp_player (cast `/Game/player/BP_Player` (`GameplayStatics.GetPlayerPawn` 0)))
  (bind _springarm (`/Game/player/BP_Player.SpringArm` _asbp_player))
  (`SceneComponent.K2_SetRelativeRotation` _springarm (`KismetMathLibrary.MakeRotator` 0.0 (`KismetMathLibrary.FClamp` (+ (* (`self.GetInputAxisKeyValue`) (`self.cameraRotationMultiply`)) (.pitch (.rotation (`SceneComponent.GetSocketTransform` _springarm "None" "RTS_World")))) -75.0) (+ (* (`self.GetInputAxisKeyValue`) (`self.cameraRotationMultiply`)) (.yaw (.rotation (`SceneComponent.GetSocketTransform` _springarm "None" "RTS_World"))))) false false))

(fn `rotatePlayer`
  (bind _asbp_player (cast `/Game/player/BP_Player` (`GameplayStatics.GetPlayerPawn` 0)))
  (bind _sphere (`/Game/player/BP_Player.Sphere` _asbp_player))
  (bind (_returnvalue_roll _returnvalue_pitch _returnvalue_yaw) (`KismetMathLibrary.BreakRotator` (`SceneComponent.GetSocketRotation` _sphere "None")))
  (`SceneComponent.K2_SetRelativeRotation` _sphere (`KismetMathLibrary.MakeRotator` 0.0 0.0 (+ _returnvalue_yaw (* (`self.GetInputAxisKeyValue`) (`self.cameraRotationMultiply`)))) false false))

(fn `UserConstructionScript`)